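; BP_SuperGlowPlatformGreen is a green platform whose appearance depends on whether the player has the MassGlow trait.
; Every tick it casts the player pawn to FirstPersonCharacter and compares its NegativeTrait and RandomTrait against "MassGlow".
; A match on either trait sets the Cube to the MI_BoostOnlyPAth material; otherwise it uses MI_DarkerGreen.
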(event `self.ReceiveTick`
  (params (DeltaSeconds :type "Float (single-precision)"))
  (bind _cube (`self.Cube`))
  ;[1 0 0] Casting
  (bind _asfirst_person_character (cast `/Game/FirstPersonBP/Blueprints/FirstPersonCharacter` (`GameplayStatics.GetPlayerCharacter` 0)))
  ;[0 1 1] Check for MassGlow
  (if (`KismetStringLibrary.EqualEqual_StrStr` "MassGlow" (`/Game/FirstPersonBP/Blueprints/FirstPersonCharacter.NegativeTrait` _asfirst_person_character))
    ;[0 1 1] Set Material
    (`PrimitiveComponent.SetMaterial` _cube 0 "/Game/MAterials/MI_BoostOnlyPAth.MI_BoostOnlyPAth" :!label _label)
    (elif (`KismetStringLibrary.EqualEqual_StrStr` "MassGlow" (`/Game/FirstPersonBP/Blueprints/FirstPersonCharacter.RandomTrait` _asfirst_person_character))
      (goto _label)
      (else
        (`PrimitiveComponent.SetMaterial` _cube 0 "/Game/MAterials/MI_DarkerGreen.MI_DarkerGreen")))))

(fn `UserConstructionScript`)