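; BP_PlatformDying is a platform that changes appearance based on the player character's traits and jump toggle.
; Tick runs through a half-second Delay, throttling polling of the FirstPersonCharacter.
; A VisionHinder random or negative trait swaps the cube to the MIIN material, with no revert.
; Otherwise, the cube's in-game visibility follows ToggleJump, hidden while true, with collision untouched.
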(event `self.ReceiveTick`
  (params (DeltaSeconds :type "Float (single-precision)"))
  (bind _cube (`self.Cube`))
  ;[1 0 0] Delay
  (`KismetSystemLibrary.Delay` 0.5)
  ;[0 1 1] Destroying the platform on limited vision
  (bind _asfirst_person_character (cast `/Game/FirstPersonBP/Blueprints/FirstPersonCharacter` (`GameplayStatics.GetPlayerCharacter` 0)))
  (if (`KismetStringLibrary.EqualEqual_StrStr` (`/Game/FirstPersonBP/Blueprints/FirstPersonCharacter.RandomTrait` _asfirst_person_character) "VisionHinder")
    (`PrimitiveComponent.SetMaterial` (`self.Cube`) 0 "/Game/MAterials/MI-IN.MI-IN" :!label _label)
    (elif (`KismetStringLibrary.EqualEqual_StrStr` "VisionHinder" (`/Game/FirstPersonBP/Blueprints/FirstPersonCharacter.NegativeTrait` _asfirst_person_character))
      (goto _label)
      (else
        ;[0 1 1] Casting - Toggle Platform according to jump
        (bind _asfirst_person_character_2 (cast `/Game/FirstPersonBP/Blueprints/FirstPersonCharacter` (`GameplayStatics.GetPlayerCharacter` 0)))
        (if (`/Game/FirstPersonBP/Blueprints/FirstPersonCharacter.ToggleJump` _asfirst_person_character_2)
          (`SceneComponent.SetHiddenInGame` _cube true false)
          (else
            (`SceneComponent.SetHiddenInGame` _cube false false)))))))

(fn `UserConstructionScript`)