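; BP_Star_Child is a star pickup, derived from a parent class, that adds to the player's score when touched.
; BeginPlay sets the actor's Tags from StartTag.
; When the player pawn overlaps Col, it adds PickUpValue to the FirstPersonCharacter's Score and prints the new star total.
; It then destroys only the collision and skeletal mesh components, leaving the actor itself in the level.
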(event `self.ReceiveBeginPlay`
  ;[1 0 0] Settings Start Tag
  (set `self.Tags` (`self.StartTag`)))

(event `self.Col.OnComponentBeginOverlap`
  (params (OverlappedComponent :type "PrimitiveComponent Object Reference") (OtherActor :type "Actor Object Reference") (OtherComp :type "PrimitiveComponent Object Reference") (OtherBodyIndex :type Integer) (bFromSweep :type Boolean) (SweepResult :type "HitResult Structure (by ref)"))
  ;[1 0 0.7] Check for colision with player
  (if (== OtherActor (`GameplayStatics.GetPlayerPawn` 0))
    ;[0.7 0 1] Casting to update the score
    (bind _asfirst_person_character (cast `/Game/FirstPersonBP/Blueprints/FirstPersonCharacter` OtherActor))
    (bind _output_get (set `/Game/FirstPersonBP/Blueprints/FirstPersonCharacter.Score` (+ (`/Game/FirstPersonBP/Blueprints/FirstPersonCharacter.Score` _asfirst_person_character) (`self.PickUpValue`)) _asfirst_person_character))
    ;[0.5 0 1] Priting the Score
    (`KismetSystemLibrary.PrintString` (`KismetStringLibrary.Concat_StrStr` "Stars: " (`KismetStringLibrary.Conv_IntToString` _output_get)))
    ;[1 0 0] Destroying Components
    (`ActorComponent.K2_DestroyComponent` (`self.Col`))
    (`ActorComponent.K2_DestroyComponent` (`self.SkeletalMesh`))))

(fn `UserConstructionScript`
  (`parent.UserConstructionScript`))